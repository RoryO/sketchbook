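; Actor that grows a phyllotaxis spiral of instanced meshes over time.
; Each Tick adds a batch of instances to a hierarchical instanced static mesh component until the step count reaches a maximum.
; Placement uses math expressions: radius is Spread times the square root of the step, angle is step times a fixed divergence angle, and height rises by a fixed increment per instance.
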(event EventBeginPlay)

(event Collision|EventActorBeginOverlap
  (params (OtherActor :type Actor%20Object%20Reference)))

(event EventTick
  (params (DeltaSeconds :type Float%20%28single-precision%29))
  (if (< (Variables|Default|GetStep) (Variables|Default|GetMax))
    (for _index (range 0 (Variables|Default|GetStride))
      (Components|InstancedStaticMesh|AddInstance (Variables|Default|GetHierarchicalInstancedStaticMesh) (CallFunction|CalculateActorPlacement))
      (Math|Integer|IncrementInt (Variables|Default|GetStep)
        (:%20%20
          (Variables|Default|SetZ%20Off (+ (Variables|Default|GetZ%20Step) (Variables|Default|GetZ%20Off))))))))

(fn ConstructionScript)

(fn CalculateActorPlacement
  (Utilities|FlowControl|Sequence
    (:then_0
      (LocalVariables|Setr (|({920BF9FA-46B4-A05D-7ED5-48B8403F3304}*(sqrt({016CF280-4611-463E-A9BD-B492AC99E257}))))))
    (:then_1
      (LocalVariables|Settheta (* (Variables|Default|GetStep) (Math|Trig|DegreesToRadians (Variables|Default|GetAngle)))))
    (:then_2
      (return (Math|Transform|MakeTransform (Math|Vector|MakeVector (|({8E69A025-43E9-7776-D531-40BB95DF4225}*(cos({62EEBF4B-483B-16CD-621D-B998F93DAD30})))) (|({8E69A025-43E9-7776-D531-40BB95DF4225}*(sin({62EEBF4B-483B-16CD-621D-B998F93DAD30})))) (Variables|Default|GetZ%20Off)))))))